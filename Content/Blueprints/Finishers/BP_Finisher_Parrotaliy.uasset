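; Parrotality finisher actor that hides the Brawl actor and replaces it with a blood burst and a slowly rising parrot.
; BeginPlay shows the Parrotality widget, spawns both effect and parrot above the CAEnemy1 component, then lifts the parrot through a looping Delay instead of Tick.
; A five-second timer removes the widget, destroys finisher and parrot, and opens the end screen with UI-only input and mouse cursor.
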(event Custom|Restart
  (bind _returnvalue (Game|GetPlayerController 0))
  (Widget|RemovefromParent (Variables|Default|GetBPW_Parrotality))
  (Actor|DestroyActor)
  (Actor|DestroyActor (Variables|Default|GetParrot))
  (bind _returnvalue_2 (UserInterface|CreateWidget "/Game/Blueprints/Widgets/BPW_End.BPW_End_C"))
  (UserInterface|Viewport|AddtoViewport _returnvalue_2 10)
  (Input|SetInputModeUIOnly _returnvalue _returnvalue_2 "DoNotLock" false)
  (Variables|/Script/Engine.PlayerController|SetbShowMouseCursor _returnvalue true))

(event EventBeginPlay
  (bind _brawl (Variables|Default|GetBrawl))
  (bind _ca_enemy1 (Variables|/Script/MyProject.Brawl|GetCA_Enemy1 _brawl))
  (bind _returnvalue (Transformation|GetWorldLocation _ca_enemy1))
  (bind _returnvalue_2 (+ _returnvalue "0.000000,0.000000,100.000000"))
  (|CallParentFunction)
  (Utilities|Time|SetTimerbyEvent (delegate Custom|Restart) 5.0)
  (bind _returnvalue_3 (UserInterface|CreateWidget "/Game/Blueprints/Widgets/BPW_Parrotality.BPW_Parrotality_C"))
  (bind _output_get (Variables|Default|SetBPW_Parrotality _returnvalue_3))
  (UserInterface|Viewport|AddtoViewport _output_get 0)
  (Rendering|SetActorHiddenInGame _brawl true)
  (Niagara|SpawnSystematLocation "/Game/Assets/Effects/Combat/NS_BloodImpact.NS_BloodImpact" _returnvalue_2 "0, 0, 0" "5.000000,5.000000,5.000000")
  (bind _returnvalue_4 (Game|SpawnActorfromClass "/Game/Blueprints/Finishers/BP_Parrot.BP_Parrot_C" (Math|Transform|MakeTransform _returnvalue_2 (Transformation|GetWorldRotation _ca_enemy1)) "AlwaysSpawn" "MultiplyWithRoot" 0 0))
  (bind _output_get_2 (Variables|Default|SetParrot _returnvalue_4))
  (Transformation|AddActorWorldOffset _output_get_2 "0.000000,0.000000,0.500000" :!label _label)
  (Utilities|FlowControl|Delay 0.03)
  (goto _label))

(event Collision|EventActorBeginOverlap
  (params (OtherActor :type Actor%20Object%20Reference))
  (|CallParentFunction OtherActor) ; This node is disabled and will not be called.\nDrag off pins to build functionality.
)

(event EventTick
  (params (DeltaSeconds :type Float%20%28single-precision%29))
  (|CallParentFunction DeltaSeconds) ; This node is disabled and will not be called.\nDrag off pins to build functionality.
)

(fn ConstructionScript
  (|CallParentFunction))
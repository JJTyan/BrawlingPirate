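; BP_Brawler is a brawler actor that drives its mesh animation from the movement of the Pawn that is its parent actor.
; Each Tick it takes that Pawn's velocity magnitude and writes it to Speed on the ABP_PunchPackV2 anim instance.
; Speed is negated unless the velocity direction points forward relative to the brawler, using a thresholded dot product, giving the animation a signed value.
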(event EventBeginPlay)

(event Collision|EventActorBeginOverlap
  (params (OtherActor :type Actor%20Object%20Reference)))

(event EventTick
  (params (DeltaSeconds :type Float%20%28single-precision%29))
  (bind _asabp_punch_pack_v2 (Utilities|Casting|CastToABP_PunchPackV2 (Components|SkeletalMesh|GetAnimInstance (Variables|Character|GetMesh))))
  (bind _aspawn (Utilities|Casting|CastToPawn (Actor|GetParentActor)))
  (Variables|/Game/Assets/PunchAnimationPackV2/Mannequin/Character/Mesh/ABP_PunchPackV2.ABP_PunchPackV2_C|SetSpeed _asabp_punch_pack_v2 (* (Math|Vector|VectorLength (Variables|/Script/Engine.MovementComponent|GetVelocity (Pawn|GetMovementComponent _aspawn))) (Math|Float|SelectFloat 1.0 -1.0 (> (Math|Vector|DotProduct (Math|Vector|Normalize (Variables|/Script/Engine.MovementComponent|GetVelocity (Pawn|GetMovementComponent _aspawn))) (Transformation|GetActorForwardVector)) 0.1)))))

(fn ConstructionScript)